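; Missile projectile Blueprint that specializes a parent class with its own impact effects.
; On BeginPlay it runs the parent logic, then assigns a grenade-launcher explosion emitter, large explosion sound, scorch decal and missile-impact sound attenuation.
; It only sets these variables and has no movement or impact logic of its own, with overlap and tick events left disabled.
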(event EventBeginPlay
  (|CallParentFunction)
  (Variables|Default|SetExplosionEmitter "/Game/BallisticsVFX/Particles/Explosive/Explosion_GrenadeLauncher_1.Explosion_GrenadeLauncher_1")
  (Variables|Default|SetHitSound "/Game/GameSoundCollection/Explosions/Cue/Large_Explosion_12_Cue.Large_Explosion_12_Cue")
  (Variables|Default|SetDecal%20Material "/Game/BallisticsVFX/Decals/Decals_Scorch.Decals_Scorch")
  (Variables|Default|SetAttenuation%20Settings "/Game/MyContent/Audio/MissileImpactsAttenuation.MissileImpactsAttenuation"))

(event Collision|EventActorBeginOverlap
  (params (OtherActor :type Actor%20Object%20Reference))
  (|CallParentFunction OtherActor) ; This node is disabled and will not be called.\nDrag off pins to build functionality.
)

(event EventTick
  (params (DeltaSeconds :type Float%20%28single-precision%29))
  (|CallParentFunction DeltaSeconds) ; This node is disabled and will not be called.\nDrag off pins to build functionality.
)

(fn ConstructionScript
  (|CallParentFunction))