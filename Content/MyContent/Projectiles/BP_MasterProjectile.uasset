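; BP_MasterProjectile is a projectile with optional homing, with launch and max speed set from variables in the construction script.
; HomingToTarget enables ProjectileMovement homing after a short retriggerable delay, and Tick turns homing missiles toward their target.
; On hit it hides visuals, plays sound and effect, applies radial falloff damage sized by Damage that ignores other projectiles, then disables collision and expires shortly after.
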(event Custom|HomingToTarget
  (params (Target :type Scene%20Component%20Object%20Reference))
  (bind _projectilemovement (Variables|Default|GetProjectileMovement))
  ;[1 1 1] SET HOMING MISSILE
  (if (Utilities|IsValid Target)
    (Variables|Default|SetHomingTarget Target)
    (Utilities|FlowControl|RetriggerableDelay 0.26)
    (Variables|/Script/Engine.ProjectileMovementComponent|SetbIsHomingProjectile _projectilemovement true)
    (Variables|/Script/Engine.ProjectileMovementComponent|SetHomingTargetComponent _projectilemovement Target)
    (Variables|/Script/Engine.ProjectileMovementComponent|SetHomingAccelerationMagnitude _projectilemovement 6e+03)))

(event EventTick
  (params (DeltaSeconds :type Float%20%28single-precision%29))
  ;[1 1 1] IF A HOMING MISSILE ALWAYS FACE TO TARGET
  (if (and (Variables|Default|GetIsHomingMissile) (Utilities|IsValid (Variables|/Script/Engine.ProjectileMovementComponent|GetHomingTargetComponent (Variables|Default|GetProjectileMovement))))
    (Transformation|SetActorRotation (Math|Interpolation|RInterpTo (Transformation|GetActorRotation) (Math|Rotator|FindLookatRotation (Transformation|GetActorLocation) (Transformation|GetWorldLocation (Variables|Default|GetHomingTarget))) (Utilities|Time|GetWorldDeltaSeconds) 2.0))))

(event Collision|EventHit
  (params (MyComp :type Primitive%20Component%20Object%20Reference) (Other :type Actor%20Object%20Reference) (OtherComp :type Primitive%20Component%20Object%20Reference) (bSelfMoved :type Boolean) (HitLocation :type Vector :default "0, 0, 0") (HitNormal :type Vector :default "0, 0, 0") (NormalImpulse :type Vector :default "0, 0, 0") (Hit :type Hit%20Result%20Structure%20%28by%20ref%29))
  (bind _returnvalue (Transformation|GetActorTransform))
  (bind _damage (Variables|Default|GetDamage))
  (bind _returnvalue_2 (Math|Float|Absolute(Float) _damage))
  ;[1 1 1] PROJECTILE HIT
  (Rendering|SetVisibility (Variables|Default|GetStaticMesh) false false)
  (Audio|SpawnSoundatLocation (Variables|Default|GetCollisionSound) HitLocation "0, 0, 0" 1.0 1.0 0.0 0 0)
  (Effects|SpawnEmitteratLocation (Variables|Default|GetCollisionFX) HitLocation (.rotation _returnvalue) (.scale _returnvalue) true "AutoRelease") ; Spawn Collision Effect
  (bind _outactors (Actor|GetAllActorsOfClass "BP_MasterProjectile_C")) ; Ignore others projectiles
  (Class|GameplayStatics|ApplyRadialDamagewithFalloff _damage (* _damage 0.3) HitLocation (* _returnvalue_2 4.0) (* _returnvalue_2 15.0) 3.0 0 _outactors self 0 "ECC_Visibility") ; Apply Damage on Hit Surface
  (Collision|SetCollisionEnabled (Variables|Default|GetPCollision) "NoCollision")
  (Actor|SetLifeSpan 0.25))

(fn ConstructionScript
  (bind _projectilemovement (Variables|Default|GetProjectileMovement))
  (Variables|/Script/Engine.ProjectileMovementComponent|SetInitialSpeed _projectilemovement (Variables|Default|GetProjectileInitSpeed))
  (Variables|/Script/Engine.ProjectileMovementComponent|SetMaxSpeed _projectilemovement (Variables|Default|GetProjectileMaxSpeed)))