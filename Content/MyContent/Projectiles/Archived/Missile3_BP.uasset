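; Missile3_BP is an archived missile projectile, a child Blueprint that relies on its parent for overlap and hit behavior.
; After the parent BeginPlay, it assigns its own explosion emitter, hit sound, impact decal and attenuation settings.
; Its overlap and hit events skip the parent handling when the other actor is a BP_MasterHeli, so the missile ignores those helicopters.
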(event EventBeginPlay
  (|CallParentFunction)
  (Variables|Default|SetExplosionEmitter "/Game/BallisticsVFX/Particles/Explosive/Explosion_Frag_small.Explosion_Frag_small")
  (Variables|Default|SetHitSound "/Game/GameSoundCollection/Explosions/Cue/Large_Explosion_03_Cue.Large_Explosion_03_Cue")
  (Variables|Default|SetDecal%20Material "/Game/BallisticsVFX/Decals/Decals__Ricochet_Gen2.Decals__Ricochet_Gen2")
  (Variables|Default|SetAttenuation%20Settings "/Game/MyContent/Audio/MissileImpactsAttenuation.MissileImpactsAttenuation"))

(event Collision|EventActorBeginOverlap
  (params (OtherActor :type Actor%20Object%20Reference))
  (Utilities|Casting|CastToBP_MasterHeli OtherActor
    (:CastFailed
      (|CallParentFunction OtherActor))))

(event Collision|EventHit
  (params (MyComp :type Primitive%20Component%20Object%20Reference) (Other :type Actor%20Object%20Reference) (OtherComp :type Primitive%20Component%20Object%20Reference) (bSelfMoved :type Boolean) (HitLocation :type Vector :default "0, 0, 0") (HitNormal :type Vector :default "0, 0, 0") (NormalImpulse :type Vector :default "0, 0, 0") (Hit :type Hit%20Result%20Structure%20%28by%20ref%29))
  (Utilities|Casting|CastToBP_MasterHeli Other
    (:CastFailed
      (|CallParentFunction MyComp Other OtherComp bSelfMoved HitLocation HitNormal NormalImpulse Hit))))

(fn ConstructionScript
  (|CallParentFunction))