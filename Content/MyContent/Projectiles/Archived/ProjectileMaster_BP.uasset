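; Archived master projectile Blueprint that explodes on landscape impact and destroys any actor it overlaps.
; A Sphere hit on a Landscape passes a DoOnce, spawns configurable explosion, sound and decal effects, then sets a short lifespan.
; The DoOnce reset follows a delay longer than that lifespan.
; Sphere overlaps print the other actor's name and destroy it immediately, with no filtering.
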(event OnComponentHit(Sphere)
  (params (HitComponent :type Primitive%20Component%20Object%20Reference) (OtherActor :type Actor%20Object%20Reference) (OtherComp :type Primitive%20Component%20Object%20Reference) (NormalImpulse :type Vector :default "0, 0, 0") (Hit :type Hit%20Result%20Structure%20%28by%20ref%29))
  (Utilities|Casting|CastToLandscape OtherActor)
  (Utilities|FlowControl|DoOnce false :!label _label
    (:Completed
      (Effects|SpawnEmitteratLocation (Variables|Default|GetExplosionEmitter) (.location Hit) "0, 0, 0" (Variables|Default|GetExplosionScale))
      (Audio|SpawnSoundatLocation (Variables|Default|GetHitSound) (.location Hit) (Transformation|GetWorldRotation (Variables|Default|GetStaticMesh)) 1.0 1.0 0.0 (Variables|Default|GetAttenuation%20Settings) 0 false)
      (Rendering|Decal|SpawnDecalatLocation (Variables|Default|GetDecal%20Material) "256.000000,256.000000,256.000000" (.location Hit) (Transformation|GetWorldRotation (Variables|Default|GetStaticMesh)) 0.0)
      (Actor|SetLifeSpan 0.2)
      (Utilities|FlowControl|Delay 2.0)
      (goto _label Reset))))

(event OnComponentBeginOverlap(Sphere)
  (params (OverlappedComponent :type Primitive%20Component%20Object%20Reference) (OtherActor :type Actor%20Object%20Reference) (OtherComp :type Primitive%20Component%20Object%20Reference) (OtherBodyIndex :type Integer) (bFromSweep :type Boolean) (SweepResult :type Hit%20Result%20Structure%20%28by%20ref%29))
  (Development|PrintString "Bullit overlapped: ")
  (Development|PrintString (Utilities|GetDisplayName OtherActor))
  (Actor|DestroyActor OtherActor))

(fn ConstructionScript)