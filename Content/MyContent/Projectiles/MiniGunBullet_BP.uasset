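; Minigun bullet projectile, a child Blueprint that leaves its impact handling to the parent class.
; On BeginPlay it runs the parent logic, then sets its own explosion emitter and scale, thud sound and soil decal, with no sound attenuation.
; Hit and overlap events ignore any BP_MasterHeli actor and pass everything else to the parent, so bullets do not react to helicopters.
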(event EventBeginPlay
  (|CallParentFunction)
  (Variables|Default|SetExplosionEmitter "/Game/BallisticsVFX/Particles/Impacts/LegacyFX/Small-Medium-Large/Asphalt/Asphalt_impact_large.Asphalt_impact_large")
  (Variables|Default|SetHitSound "/Game/BallisticsVFX/SFX/Impacts/Generic/Thud_1.Thud_1")
  (Variables|Default|SetDecal%20Material "/Game/BallisticsVFX/Decals/Decals_Soil.Decals_Soil")
  (Variables|Default|SetAttenuation%20Settings 0)
  (Variables|Default|SetExplosionScale "5.000000,5.000000,5.000000"))

(event EventTick
  (params (DeltaSeconds :type Float%20%28single-precision%29))
  (|CallParentFunction DeltaSeconds) ; This node is disabled and will not be called.\nDrag off pins to build functionality.
)

(event Collision|EventHit
  (params (MyComp :type Primitive%20Component%20Object%20Reference) (Other :type Actor%20Object%20Reference) (OtherComp :type Primitive%20Component%20Object%20Reference) (bSelfMoved :type Boolean) (HitLocation :type Vector :default "0, 0, 0") (HitNormal :type Vector :default "0, 0, 0") (NormalImpulse :type Vector :default "0, 0, 0") (Hit :type Hit%20Result%20Structure%20%28by%20ref%29))
  (Utilities|Casting|CastToBP_MasterHeli Other
    (:CastFailed
      (|CallParentFunction MyComp Other OtherComp bSelfMoved HitLocation HitNormal NormalImpulse Hit))))

(event Collision|EventActorBeginOverlap
  (params (OtherActor :type Actor%20Object%20Reference))
  (Utilities|Casting|CastToBP_MasterHeli OtherActor
    (:CastFailed
      (|CallParentFunction OtherActor))))

(fn ConstructionScript
  (|CallParentFunction))