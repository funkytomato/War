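; WarGameMode is a game mode Blueprint that keeps a running count of elapsed level time.
; BeginPlay starts a looping one-second timer that calls LevelTimer by function name, so Tick stays unused.
; LevelTimer increments Seconds and rolls it over into Minutes after 59, with no upper limit or display logic in the graph.
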(event EventBeginPlay
  (Utilities|Time|SetTimerbyFunctionName 0 "LevelTimer" 1.0 true))

(event EventTick
  (params (DeltaSeconds :type Float%20%28single-precision%29)))

(fn ConstructionScript)

(fn LevelTimer
  (Variables|Default|SetSeconds (+ (Variables|Default|GetSeconds) 1))
  (if (> (Variables|Default|GetSeconds) 59)
    (Variables|Default|SetMinutes (+ (Variables|Default|GetMinutes) 1))
    (Variables|Default|SetSeconds 0)))