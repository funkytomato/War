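; Base turret actor that detects helicopters (BP_MasterHeli) entering a radius-configurable sphere, then tracks and shoots them.
; A looping aim timer interpolates GunRotator toward the target with accelerating turn speed and clamped pitch, then line-traces from the muzzle.
; DoOnce gates toggle a fire-rate timer that spawns BP_MasterProjectile while the line of sight is clear.
; Incoming damage, including projectile critical damage, is forwarded to BPDamageComponent.
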(event OnComponentBeginOverlap(DetectionRadar)
  (params (OverlappedComponent :type Primitive%20Component%20Object%20Reference) (OtherActor :type Actor%20Object%20Reference) (OtherComp :type Primitive%20Component%20Object%20Reference) (OtherBodyIndex :type Integer) (bFromSweep :type Boolean) (SweepResult :type Hit%20Result%20Structure%20%28by%20ref%29))
  (bind _asbp_master_heli (Utilities|Casting|CastToBP_MasterHeli OtherActor))
  (Variables|Default|SetTargetInRange true)
  (CallFunction|AcquireTarget _asbp_master_heli))

(event OnComponentEndOverlap(DetectionRadar)
  (params (OverlappedComponent :type Primitive%20Component%20Object%20Reference) (OtherActor :type Actor%20Object%20Reference) (OtherComp :type Primitive%20Component%20Object%20Reference) (OtherBodyIndex :type Integer))
  (Utilities|Casting|CastToBP_MasterHeli OtherActor)
  (Variables|Default|SetTargetInRange false)
  (Utilities|Time|ClearTimerbyFunctionName 0 "FireUponTarget")
  (CallFunction|ResetTargetOutOfRangeDoOnce)
  (CallFunction|ResetTargetHitDoOnce))

(event Custom|AcquireTarget
  (params (TargetRef :type Actor%20Object%20Reference))
  (Variables|Default|SetTargetReference TargetRef)
  (Utilities|Time|SetTimerbyFunctionName self "AimAtTarget" (Variables|Default|GetAiming%20Update%20Interval) true)
  (CallFunction|ResetTargetOutOfRangeDoOnce))

(event Custom|AimAtTarget
  (bind _targetreference (Variables|Default|GetTargetReference))
  (bind _returnvalue (Transformation|GetActorLocation _targetreference))
  (bind (_x _y _z) (Math|Vector|BreakVector _returnvalue))
  (Utilities|IsValid (Variables|Default|GetTargetReference)
    (:Is%20Valid
      (bind _y_n (Class|BPIHeliInterface|IsDead?(Message) (Variables|Default|GetTargetReference)))
      (if (and (not _y_n) (Variables|Default|GetTargetInRange))
        (Utilities|FlowControl|Sequence
          (:then_0
            (CallFunction|RotateTowardsTarget))
          (:then_1
            (bind _outhit (Collision|LineTraceForObjects (Transformation|GetSocketLocation (Variables|Default|GetSKMesh) "Muzzle") (Math|Vector|MakeVector _x _y (+ _z 5e+01)) (Utilities|Array|MakeArray "ObjectTypeQuery3" "ObjectTypeQuery1") false (Utilities|Array|MakeArray (Variables|Default|GetBulletRef)) "None" true "(R=1.000000,G=0.000000,B=0.000000,A=1.000000)" "(R=0.000000,G=1.000000,B=0.000000,A=1.000000)" 1.0))
            (Variables|Default|SetBlockedByPlayer (== (.HitActor (Collision|BreakHitResult _outhit)) (Variables|Default|GetTargetReference)))
            (if (Variables|Default|GetBlockedByPlayer)
              (Utilities|FlowControl|DoOnce false
                (:Completed
                  (Utilities|Time|SetTimerbyFunctionName self "FireUponTarget" (/ 1.0 (Variables|Default|GetFire%20Rate)) true)))
              (else
                (CallFunction|ResetTargetHitDoOnce)
                (Utilities|Time|ClearTimerbyFunctionName 0 "FireUponTarget")))))
        (else
          (Utilities|FlowControl|DoOnce false
            (:Completed
              (Utilities|Time|ClearTimerbyFunctionName 0 "AimAtTarget"))))))))

(event Custom|FireUponTarget
  (bind _skmesh (Variables|Default|GetSKMesh))
  (bind _returnvalue (Transformation|GetSocketTransform _skmesh "Muzzle" "RTS_World"))
  (bind _returnvalue_2 (Game|SpawnActorfromClass "/Game/MyContent/Projectiles/BP_MasterProjectile.BP_MasterProjectile_C" (Math|Transform|MakeTransform (.location _returnvalue) (.rotation _returnvalue) "1,1,1") "Undefined" 0 5e+03 9e+03 false 0.0 false 0))
  (Variables|Default|SetBulletRef _returnvalue_2))

(event Custom|Reset%20Target%20Hit%20DoOnce
  (Utilities|FlowControl|DoOnce false) ; enters at Reset
)

(event Custom|Reset%20Target%20OutOfRange%20Do%20Once
  (Utilities|FlowControl|DoOnce false) ; enters at Reset
)

(event Game|Damage|EventAnyDamage
  (params (Damage :type Float%20%28single-precision%29) (DamageType :type Damage%20Type%20Object%20Reference) (InstigatedBy :type Controller%20Object%20Reference) (DamageCauser :type Actor%20Object%20Reference))
  (Default|ReceiveDamage (Variables|Default|GetBP_DamageComponent) self Damage (Variables|/Game/MyContent/Projectiles/BP_MasterProjectile.BP_MasterProjectile_C|GetCriticalDamage (.AsBP%20Master%20Projectile (Utilities|Casting|CastToBP_MasterProjectile DamageCauser)))))

(event EventBeginPlay
  (bind _bp_damagecomponent (Variables|Default|GetBP_DamageComponent))
  (Variables|/Game/ArcadeHelicopter/Blueprints/Components/BP_DamageComponent.BP_DamageComponent_C|SetHealth _bp_damagecomponent 1e+02)
  (Variables|/Game/ArcadeHelicopter/Blueprints/Components/BP_DamageComponent.BP_DamageComponent_C|SetArmorPercentage _bp_damagecomponent 1e+01))

(fn ConstructionScript
  (Components|Sphere|SetSphereRadius (Variables|Default|GetDetectionRadar) (Variables|Default|GetDetectionRange) true))

(fn RotateTowardsTarget
  (bind _skmesh (Variables|Default|GetSKMesh))
  (Variables|Default|SetCurrent%20Rotation%20Speed (Math|Interpolation|FInterpTo (Variables|Default|GetCurrent%20Rotation%20Speed) (Variables|Default|GetMax%20Rotation%20Speed) (Utilities|Time|GetWorldDeltaSeconds) 1.0))
  (Variables|Default|SetGunRotator (Math|Interpolation|RInterpTo (Variables|Default|GetGunRotator) (Math|Rotator|MakeRotator (.Roll (Math|Rotator|BreakRotator (Transformation|GetSocketRotation _skmesh "Main"))) (Math|Float|ClampAngle (.Pitch (Math|Rotator|BreakRotator (Math|Rotator|FindLookatRotation (Transformation|GetSocketLocation _skmesh "Barrel") (Transformation|GetActorLocation (Variables|Default|GetTargetReference))))) (Variables|Default|GetHead%20Min%20Pitch) (Variables|Default|GetHead%20Max%20Pitch)) (.Yaw (Math|Rotator|BreakRotator (Math|Rotator|FindLookatRotation (Transformation|GetSocketLocation _skmesh "Main") (Transformation|GetActorLocation (Variables|Default|GetTargetReference)))))) (Utilities|Time|GetWorldDeltaSeconds) (Variables|Default|GetCurrent%20Rotation%20Speed))))

(fn IsDead?
  (return false))