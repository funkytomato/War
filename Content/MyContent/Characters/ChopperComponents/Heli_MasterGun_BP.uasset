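; Base gun Blueprint for the war helicopter that fires projectiles and projects an aiming reticle decal, with firing specifics left to subclasses.
; A looping timer traces forward from the gun and moves the decal to the hit point.
; FireGun checks the instigating helicopter's trigger, then spawns the projectile class at the arrow until the magazine limit is reached.
; The next fire attempt resets the shot count and blocks firing during a short reload delay.
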(event Custom|FireRayTrace
  (bind _decal (Variables|Default|GetDecal))
  (bind _gun (Variables|Default|GetGun))
  (bind _returnvalue (Transformation|GetWorldLocation _gun))
  ;[1 1 1] Fire Ray Trace
  (bind (_outhit _returnvalue_2) (Collision|LineTraceByChannel _returnvalue (+ _returnvalue (* (Math|Vector|GetForwardVector (Transformation|GetWorldRotation _gun)) (Variables|Default|GetRayTraceRange))) "TraceTypeQuery1" false 0 "None" true "(R=1.000000,G=0.000000,B=0.000000,A=1.000000)" "(R=0.875709,G=0.109517,B=1.000000,A=1.000000)" 0.5))
  (if _returnvalue_2
    (Transformation|SetWorldLocation _decal (.location _outhit) false true)
    (Transformation|SetWorldRotation _decal (Transformation|GetWorldRotation (Variables|Default|GetGun)) false false)))

(event Custom|FireGun
  ;[1 1 1] Fire Gun, Projectile fire is defined in the subclass
  (if (Variables|Default|GetCanFire)
    (bind _aswar_helicopter_bp (Utilities|Casting|CastToWarHelicopter_BP (Game|GetInstigator)))
    (if (Variables|/Game/MyContent/Characters/WarHelicopter_BP.WarHelicopter_BP_C|GetFireTriggerPressed _aswar_helicopter_bp)
      (if (< (Variables|Default|GetShotsFired) (Variables|Default|GetMagSize))
        (Game|SpawnActorfromClass (Variables|Default|GetProjectileClass) (Transformation|GetWorldTransform (Variables|Default|GetArrow)) "DontSpawnIfColliding" 0 (Variables|Actor|GetInstigator))
        (Variables|Default|SetShotsFired (+ (Variables|Default|GetShotsFired) 1))
        (else
          (Variables|Default|SetShotsFired 0)
          (Variables|Default|SetCanFire false)
          (Utilities|FlowControl|Delay 1.0)
          (Variables|Default|SetCanFire true))))))

(event EventBeginPlay
  (bind _decal (Variables|Default|GetDecal))
  ;[1 1 1] Start Timer for RayTrace and set the location and rotation of the retina Decal
  (Utilities|Time|SetTimerbyFunctionName 0 "FireRayTrace" 0.2 true)
  (Transformation|SetWorldLocation _decal (Variables|Default|GetRetinaDecalLocation) false true)
  (Transformation|SetWorldRotation _decal "0,180.000000, 0" false false))

(fn ConstructionScript)