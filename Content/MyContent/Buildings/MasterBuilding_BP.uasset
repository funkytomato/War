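; MasterBuilding_BP is a damageable building Blueprint, by its name the base for the game's buildings.
; On AnyDamage it casts the damage causer to BP_MasterProjectile and passes the damage and critical damage to BPDamageComponent.
; When the component reports destroyed, the structure mesh swaps to a fixed destroyed barracks mesh and a burning effect plays for a short delay before deactivating.
; Damage from other causers is ignored, and debug strings print on hit and destruction.
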(event EventBeginPlay)

(event Collision|EventActorBeginOverlap
  (params (OtherActor :type Actor%20Object%20Reference)))

(event EventTick
  (params (DeltaSeconds :type Float%20%28single-precision%29)))

(event Game|Damage|EventAnyDamage
  (params (Damage :type Float%20%28single-precision%29) (DamageType :type Damage%20Type%20Object%20Reference) (InstigatedBy :type Controller%20Object%20Reference) (DamageCauser :type Actor%20Object%20Reference))
  (bind _burningfx (Variables|Default|GetBurningFX))
  (Development|PrintString "recieving damage")
  (bind _asbp_master_projectile (Utilities|Casting|CastToBP_MasterProjectile DamageCauser))
  (Default|ReceiveDamage (Variables|Default|GetBP_DamageComponent) self Damage (Variables|/Game/MyContent/Projectiles/BP_MasterProjectile.BP_MasterProjectile_C|GetCriticalDamage _asbp_master_projectile))
  (if (Variables|/Game/MyContent/Characters/ArcadeHeli/BP_DamageComponent.BP_DamageComponent_C|GetIsDestroyed (Variables|Default|GetBP_DamageComponent))
    (Development|PrintString "Is Destroyed")
    (Components|StaticMesh|SetStaticMesh (Variables|Default|GetStructureMesh) "/Game/PolygonMilitary/Meshes/Buildings/SM_Bld_Barracks_Destroyed_01.SM_Bld_Barracks_Destroyed_01")
    (Components|Activation|Activate _burningfx false)
    (Utilities|FlowControl|Delay 2.0)
    (Components|Activation|Deactivate _burningfx)))

(fn ConstructionScript)