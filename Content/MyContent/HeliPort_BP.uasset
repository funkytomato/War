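; Helipad actor that refuels, rearms and repairs a BP_MasterHeli landed on it.
; Entering CanLandCollision notifies the helicopter it can land and starts, via a DoOnce, a looping timer polling LandedCollision.
; While the first overlapping helicopter reports CanLand and IsLanded, each tick tops up fuel and ammo and reduces damage on the stored helicopter reference.
; Leaving CanLandCollision revokes landing, clears the timer and resets the DoOnce.
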(event OnComponentBeginOverlap(CanLandCollision)
  (params (OverlappedComponent :type Primitive%20Component%20Object%20Reference) (OtherActor :type Actor%20Object%20Reference) (OtherComp :type Primitive%20Component%20Object%20Reference) (OtherBodyIndex :type Integer) (bFromSweep :type Boolean) (SweepResult :type Hit%20Result%20Structure%20%28by%20ref%29))
  (bind _asbp_master_heli (Utilities|Casting|CastToBP_MasterHeli OtherActor))
  (Utilities|IsValid _asbp_master_heli
    (:Is%20Valid
      (Variables|Default|SetMasterHeliRef _asbp_master_heli)
      (Default|CallCanLandMsg _asbp_master_heli self)
      (Utilities|FlowControl|DoOnce false
        (:Completed
          (bind _returnvalue (Utilities|Time|SetTimerbyFunctionName 0 "CheckHeliLanded" 0.2 true))
          (Variables|Default|SetCheckLandedTimerRef _returnvalue))))))

(event OnComponentEndOverlap(CanLandCollision)
  (params (OverlappedComponent :type Primitive%20Component%20Object%20Reference) (OtherActor :type Actor%20Object%20Reference) (OtherComp :type Primitive%20Component%20Object%20Reference) (OtherBodyIndex :type Integer))
  (bind _asbp_master_heli (Utilities|Casting|CastToBP_MasterHeli OtherActor))
  (Utilities|IsValid _asbp_master_heli
    (:Is%20Valid
      (Default|CallNoLandMsg _asbp_master_heli)
      (Utilities|Time|ClearandInvalidateTimerbyHandle (Variables|Default|GetCheckLandedTimerRef))
      (Utilities|FlowControl|DoOnce false) ; enters at Reset
    )))

(fn ConstructionScript)

(fn CheckHeliLanded
  (bind _asbp_master_heli (Utilities|Casting|CastToBP_MasterHeli (Utilities|Array|Get(acopy) (Collision|GetOverlappingActors (Variables|Default|GetLandedCollision) "/Game/MyContent/Characters/ArcadeHeli/BP_MasterHeli.BP_MasterHeli_C" :!class /Script/Engine.PrimitiveComponent))))
  (if (Variables|/Game/MyContent/Characters/ArcadeHeli/BP_MasterHeli.BP_MasterHeli_C|GetCanLand _asbp_master_heli)
    (if (Variables|/Game/MyContent/Characters/ArcadeHeli/BP_MasterHeli.BP_MasterHeli_C|GetIsLanded _asbp_master_heli)
      (CallFunction|MaintainHelicopter))))

(fn MaintainHelicopter
  (Default|CallIncreaseFuel (Variables|Default|GetMasterHeliRef) 100)
  (Default|CallIncreaseAmmo (Variables|Default|GetMasterHeliRef) 999)
  (Default|CallDecreaseDamage (Variables|Default|GetMasterHeliRef) 100))